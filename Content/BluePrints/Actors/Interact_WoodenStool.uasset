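; Interactable wooden stool whose cover swings open for the player once the CATHY unlock is set on MainCharacter.
; On overlap, an unlocked player triggers a timeline that rotates Cover, and leaving reverses it.
; Otherwise it shows an E prompt and opens a gate, letting Interact spawn a CharacterLock widget that receives the player and stool.
; A separate Open event plays the same timeline.
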(event `InputAction|Interact`
  (params (Key :type "Key Structure"))
  ;[1 1 1] Press E Key to show character lock if isUnlocked is false
  (:`Pressed`
    (`/Engine/EditorBlueprintResources/StandardMacros.Gate` true :!label _label
      (:`Exit`
        (bind _returnvalue (`|CreateWidget` "/Game/BluePrints/Widget/CharacterLock.CharacterLock_C"))
        (`/Game/BluePrints/Widget/CharacterLock.setRefActors` _returnvalue (`self.MainActor`) self)
        (`UserWidget.AddToViewport` _returnvalue 0)
        (`Widget.RemoveFromParent` (stale `self.ReceiveActorBeginOverlap` _returnvalue))))))

(event `self.ReceiveActorBeginOverlap`
  (params (OtherActor :type "Actor Object Reference"))
  (bind _asmain_character (cast `/Game/BluePrints/Actors/MainCharacter` OtherActor))
  (set `self.MainActor` _asmain_character)
  (if (`/Game/BluePrints/Actors/MainCharacter.isUnlocked_CATHY` (`self.MainActor`))
    ;[1 1 1] Move stool if isUnlocked is true
    (bind (_direction _move) (`Timeline|타임라인_0` :!via `PlayFromStart` :!label _label_2)
      (:`Update`
        (`SceneComponent.K2_SetRelativeRotation` (`self.Cover`) (`KismetMathLibrary.MakeRotator` (`KismetMathLibrary.Lerp` 0.0 -90.0 _move)) false false)))
    (else
      (`|ExecutionSequence`
        (:`then_0`
          (goto _label :!via `Open`))
        (:`then_1`
          ;[1 1 1] add/remove widget of E interact
          (bind _returnvalue (`|CreateWidget` "/Game/BluePrints/Widget/InteractKeyPrompt_E.InteractKeyPrompt_E_C"))
          (`UserWidget.AddToViewport` _returnvalue 0)
          (`self.EnableInput` (`GameplayStatics.GetPlayerController` 0)))))))

(event `self.ReceiveActorEndOverlap`
  (params (OtherActor :type "Actor Object Reference"))
  (if (`/Game/BluePrints/Actors/MainCharacter.isUnlocked_CATHY` (`self.MainActor`))
    (`|ExecutionSequence`
      (:`then_0`
        (goto _label :!via `Close`))
      (:`then_1`
        (goto _label_2 :!via `Reverse`)))
    (else
      (`|ExecutionSequence`
        (:`then_0`
          (goto _label :!via `Close`))
        (:`then_1`
          ;[1 1 1] add/remove widget of E interact
          (`Widget.RemoveFromParent` (stale `self.ReceiveActorBeginOverlap` _returnvalue))
          (`self.DisableInput` (`GameplayStatics.GetPlayerController` 0)))))))

(event `Open`
  (goto _label_2 :!via `PlayFromStart`))

(fn `UserConstructionScript`)