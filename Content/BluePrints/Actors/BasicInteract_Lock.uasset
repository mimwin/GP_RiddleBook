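; BasicInteract_Lock is an interactable lock actor that shows a digit lock UI when the player interacts with it nearby.
; Beginning an overlap creates an E-key prompt widget, enables input for player controller 0 and opens a Gate; ending it reverses this.
; Pressing Interact passes through that Gate to add a new DigitLock2 widget to the viewport and remove the prompt.
; Overlaps are not filtered by actor.
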(event `InputAction|Interact`
  (params (Key :type "Key Structure"))
  ;[1 1 1] Press E Key to move
  (:`Pressed`
    (`/Engine/EditorBlueprintResources/StandardMacros.Gate` true :!label _label
      (:`Exit`
        (bind _returnvalue (`|CreateWidget` "/Game/BluePrints/Widget/DigitLock2.DigitLock2_C"))
        (`UserWidget.AddToViewport` _returnvalue 0)
        (`Widget.RemoveFromParent` (stale `self.ReceiveActorBeginOverlap` _returnvalue))))))

(event `self.ReceiveActorBeginOverlap`
  (params (OtherActor :type "Actor Object Reference"))
  ;[1 1 1] add/remove widget and enable/disable input
  (bind _returnvalue (`|CreateWidget` "/Game/BluePrints/Widget/InteractKeyPrompt_E.InteractKeyPrompt_E_C"))
  (`UserWidget.AddToViewport` _returnvalue 0)
  (`self.EnableInput` (`GameplayStatics.GetPlayerController` 0))
  (goto _label :!via `Open`))

(event `self.ReceiveActorEndOverlap`
  (params (OtherActor :type "Actor Object Reference"))
  ;[1 1 1] add/remove widget and enable/disable input
  (`Widget.RemoveFromParent` (stale `self.ReceiveActorBeginOverlap` _returnvalue))
  (`self.DisableInput` (`GameplayStatics.GetPlayerController` 0))
  (goto _label :!via `Close`))

(fn `UserConstructionScript`)