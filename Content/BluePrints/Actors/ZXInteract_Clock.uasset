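; Interactable clock puzzle that grants the player a key when its hands are stepped to a target position.
; Overlap shows a subtitle and, until the key is obtained, an E prompt that unlocks X and Z to turn the hour and minute hands with sound.
; Gates control input; key releases increment counters checked modulo 12, setting IsKeyObtained on MainCharacter and briefly showing an item subtitle.
; Leaving closes the hand gates and removes prompts.
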(event `CheckValue`
  ;[1 1 1] check time to get Key
  (if (`/Game/BluePrints/Actors/MainCharacter.isKeyObtained` (`self.MainActor`))
    _
    (elif (and (== (mod (`KismetMathLibrary.Conv_Int64ToInt` (`self.Hour_cnt`)) 12) 1) (== (mod (`KismetMathLibrary.Conv_Int64ToInt` (`self.Min_cnt`)) 12) 10))
      ;;[1 1 1] set isKeyObtained - (2)
      (set `/Game/BluePrints/Actors/MainCharacter.isKeyObtained` true (`self.MainActor`))
      ;[1 1 1] Item Subtitle : You got the key! (Key Obtained)
      (bind _returnvalue (`|CreateWidget` "/Game/BluePrints/Widget/Item_Subtitles.Item_Subtitles_C"))
      (bind _output_get (set `self.ItemSubtitleWidgetRef` _returnvalue))
      (`UserWidget.AddToViewport` _output_get 0)
      (`self.Item Subtitle Text`)
      (`KismetSystemLibrary.Delay` 4.0)
      (`Widget.RemoveFromParent` _output_get))))

(event `Item Subtitle Text`
  ;[1 1 1] Item Subtitle : You got the key! (Key Obtained)
  (`/Game/BluePrints/Widget/Item_Subtitles.DisplayItemLine` (`self.ItemSubtitleWidgetRef`) "You got the key!"))

(event `Subtitle Text`
  ;[1 1 1] Subtitle - It's a clock
  (`/Game/BluePrints/Widget/Subtitles.DisplayLine` (`self.SubtitlesWidgetRef`) "Oh... It's a clock."))

(event `self.ReceiveActorBeginOverlap`
  (params (OtherActor :type "Actor Object Reference"))
  (bind _clock_hour (`self.Clock_Hour`))
  (bind _clock_min (`self.Clock_Min`))
  ;[1 1 1] add widget and enable input
  (bind _asmain_character (cast `/Game/BluePrints/Actors/MainCharacter` OtherActor))
  (bind _output_get (set `self.MainActor` _asmain_character))
  (`|ExecutionSequence`
    (:`then_0`
      (bind _returnvalue (`|CreateWidget` "/Game/BluePrints/Widget/Subtitles.Subtitles_C"))
      (bind _output_get_2 (set `self.SubtitlesWidgetRef` _returnvalue))
      (`self.Subtitle Text`)
      (`UserWidget.AddToViewport` _output_get_2 0))
    (:`then_1`
      (if (not (`/Game/BluePrints/Actors/MainCharacter.isKeyObtained` _output_get))
        (bind _returnvalue_2 (`|CreateWidget` "/Game/BluePrints/Widget/InteractKeyPrompt_E.InteractKeyPrompt_E_C"))
        (bind _output_get_3 (set `self.InteractEWidget` _returnvalue_2))
        (`UserWidget.AddToViewport` _output_get_3 0)
        (`self.EnableInput` (`GameplayStatics.GetPlayerController` 0))
        (goto _label_2 :!via `Open`)))))

(event `Key|X`
  (params (Key :type "Key Structure"))
  (bind _clock_hour (`self.Clock_Hour`))
  ;[1 1 1] Press x key for moving HOUR
  (:`Pressed`
    (`/Engine/EditorBlueprintResources/StandardMacros.Gate` true :!label _label
      (:`Exit`
        (bind _returnvalue (`GameplayStatics.SpawnSound2D` "/Game/Assets/Audio/clock_hand.clock_hand" 1.0 1.0 0.0 null))
        (set `self.2dSound` _returnvalue)
        (`SceneComponent.K2_SetRelativeRotation` _clock_hour (`KismetMathLibrary.MakeRotator` (.roll (`SceneComponent.RelativeRotation` _clock_hour)) (.pitch (`SceneComponent.RelativeRotation` _clock_hour)) (+ (.yaw (`SceneComponent.RelativeRotation` _clock_hour)) 30.0)) false false))))
  (:`Released`
    ;[1 1 1] count Clock_Hour move and check
    (if (`self.isEpressed`)
      (set `self.Hour_cnt` (+ (`self.Hour_cnt`) 1))
      (`self.CheckValue`))))

(event `InputAction|Interact`
  (params (Key :type "Key Structure"))
  (bind _clock_min (`self.Clock_Min`))
  ;[1 1 1] open/close gate for Interact Input Action (E key)
  (:`Pressed`
    (`/Engine/EditorBlueprintResources/StandardMacros.Gate` true :!label _label_2
      (:`Exit`
        (set `self.isEpressed` true)
        (`Widget.RemoveFromParent` (`self.SubtitlesWidgetRef`))
        (`Widget.RemoveFromParent` (`self.InteractEWidget`))
        (`|ExecutionSequence`
          (:`then_0`
            ;[1 1 1] add Interact ZX key widget
            (bind _returnvalue (`|CreateWidget` "/Game/BluePrints/Widget/InteractKeyPrompt_ZX.InteractKeyPrompt_ZX_C"))
            (set `self.InteractZXWidget` _returnvalue)
            (`UserWidget.AddToViewport` _returnvalue 0)
            (`|ExecutionSequence`
              (:`then_0`
                (goto _label :!via `Open`))
              (:`then_1`
                (goto _label_3 :!via `Open`))))
          (:`then_1`
            (goto _label_2 :!via `Close`)))))))

(event `self.ReceiveActorEndOverlap`
  (params (OtherActor :type "Actor Object Reference"))
  (bind _interactzxwidget (`self.InteractZXWidget`))
  (bind _subtitleswidgetref (`self.SubtitlesWidgetRef`))
  (bind _clock_min (`self.Clock_Min`))
  ;[1 1 1] remove valid widget and disable input
  (`|ExecutionSequence`
    (:`then_0`
      (`self.DisableInput` (`GameplayStatics.GetPlayerController` 0))
      (`|ExecutionSequence`
        (:`then_0`
          (goto _label :!via `Close`))
        (:`then_1`
          (goto _label_3 :!via `Close`))))
    (:`then_1`
      (if (`KismetSystemLibrary.IsValid` _interactzxwidget)
        (`Widget.RemoveFromParent` _interactzxwidget)))
    (:`then_2`
      (if (`KismetSystemLibrary.IsValid` _subtitleswidgetref)
        (`Widget.RemoveFromParent` _subtitleswidgetref)
        (`Widget.RemoveFromParent` (`self.InteractEWidget`))))))

(event `Key|Z`
  (params (Key :type "Key Structure"))
  (bind _clock_min (`self.Clock_Min`))
  ;[1 1 1] Press z key for moving MINUTE
  (:`Pressed`
    (`/Engine/EditorBlueprintResources/StandardMacros.Gate` true :!label _label_3
      (:`Exit`
        (bind _returnvalue (`GameplayStatics.SpawnSound2D` "/Game/Assets/Audio/clock_hand.clock_hand" 1.0 1.0 0.0 null))
        (set `self.2dSound` _returnvalue)
        (`SceneComponent.K2_SetRelativeRotation` _clock_min (`KismetMathLibrary.MakeRotator` (.roll (`SceneComponent.RelativeRotation` _clock_min)) (.pitch (`SceneComponent.RelativeRotation` _clock_min)) (+ (.yaw (`SceneComponent.RelativeRotation` _clock_min)) 30.0)) false false))))
  (:`Released`
    ;[1 1 1] Count Clock_Min move and check
    (if (`self.isEpressed`)
      (set `self.Min_cnt` (+ (`self.Min_cnt`) 1))
      (`self.CheckValue`))))

(fn `UserConstructionScript`)