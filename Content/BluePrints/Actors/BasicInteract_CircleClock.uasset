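; Interactable circle clock actor that rotates clock ring actors from key presses while the player overlaps it.
; Overlap shows an E prompt, enables input and opens a gate; leaving reverses all three.
; X passes through that gate to roll ClockCircleB's owner with debug prints, while Z rolls ClockCircleC's owner by a smaller step.
; The Interact action adds a DigitLock2 widget to the viewport through a Gate.
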(event `InputAction|Interact`
  (params (Key :type "Key Structure"))
  ;[1 1 1] Press E Key to move
  (:`Pressed`
    ;[1 1 1] Open/Close Gate
    (`/Engine/EditorBlueprintResources/StandardMacros.Gate` true
      (:`Exit`
        (bind _returnvalue (`|CreateWidget` "/Game/BluePrints/Widget/DigitLock2.DigitLock2_C"))
        (`UserWidget.AddToViewport` _returnvalue 0)))))

(event `self.ReceiveActorBeginOverlap`
  (params (OtherActor :type "Actor Object Reference"))
  (bind _returnvalue (`KismetMathLibrary.MakeRotator` (+ (.roll (`self.K2_GetActorRotation` (`ActorComponent.GetOwner` (`self.ClockCircle_B`)))) 50.0) (.pitch (`self.K2_GetActorRotation` (`ActorComponent.GetOwner` (`self.ClockCircle_B`)))) (.yaw (`self.K2_GetActorRotation` (`ActorComponent.GetOwner` (`self.ClockCircle_B`))))))
  ;[1 1 1] add/remove widget and enable/disable input
  (bind _returnvalue_2 (`|CreateWidget` "/Game/BluePrints/Widget/InteractKeyPrompt_E.InteractKeyPrompt_E_C"))
  (`UserWidget.AddToViewport` _returnvalue_2 0)
  (`self.EnableInput` (`GameplayStatics.GetPlayerController` 0))
  (goto _label :!via `Open`))

(event `Key|X`
  (params (Key :type "Key Structure"))
  (bind _returnvalue (`KismetMathLibrary.MakeRotator` (+ (.roll (`self.K2_GetActorRotation` (`ActorComponent.GetOwner` (`self.ClockCircle_B`)))) 50.0) (.pitch (`self.K2_GetActorRotation` (`ActorComponent.GetOwner` (`self.ClockCircle_B`)))) (.yaw (`self.K2_GetActorRotation` (`ActorComponent.GetOwner` (`self.ClockCircle_B`))))))
  (:`Pressed`
    (`/Engine/EditorBlueprintResources/StandardMacros.Gate` true :!label _label
      (:`Exit`
        (bind _returnvalue_2 (`self.K2_SetActorRotation` (`ActorComponent.GetOwner` (`self.ClockCircle_B`)) _returnvalue false))
        (`KismetSystemLibrary.PrintText` "Hello")
        (`KismetSystemLibrary.PrintText` (`KismetTextLibrary.Conv_BoolToText` _returnvalue_2))
        (`KismetSystemLibrary.PrintText` (`KismetTextLibrary.Conv_RotatorToText` _returnvalue))))))

(event `self.ReceiveActorEndOverlap`
  (params (OtherActor :type "Actor Object Reference"))
  ;[1 1 1] add/remove widget and enable/disable input
  (`Widget.RemoveFromParent` (stale `self.ReceiveActorBeginOverlap` _returnvalue_2))
  (`self.DisableInput` (`GameplayStatics.GetPlayerController` 0))
  (goto _label :!via `Close`))

(event `Key|Z`
  (params (Key :type "Key Structure"))
  (:`Pressed`
    (`self.K2_SetActorRotation` (`ActorComponent.GetOwner` (`self.ClockCircle_C`)) (`KismetMathLibrary.MakeRotator` (+ (.roll (`self.K2_GetActorRotation` (`ActorComponent.GetOwner` (`self.ClockCircle_C`)))) 6.0) (.pitch (`self.K2_GetActorRotation` (`ActorComponent.GetOwner` (`self.ClockCircle_C`)))) (.yaw (`self.K2_GetActorRotation` (`ActorComponent.GetOwner` (`self.ClockCircle_C`))))) false)))

(fn `UserConstructionScript`)