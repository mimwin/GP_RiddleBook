(event `InputAction|Interact`
  (params (Key :type "Key Structure"))
  ;[1 1 1] Press E Key to move
  (:`Pressed`
    (`/Engine/EditorBlueprintResources/StandardMacros.Gate` true :!label _label
      (:`Exit`
        (`Widget.RemoveFromParent` (stale `self.ReceiveActorBeginOverlap` _returnvalue))
        ;[1 1 1] if isDrugFound is true then show Drug widget, else show digitlock widget
        (if (`/Game/BluePrints/Actors/MainCharacter.isDrugFound` (`self.MainActor`))
          (`self.SelectDrug`)
          (else
            (bind _returnvalue (`|CreateWidget` "/Game/BluePrints/Widget/DigitLock2.DigitLock2_C"))
            (`/Game/BluePrints/Widget/DigitLock2.setRefActors` _returnvalue (`self.MainActor`) self)
            (`UserWidget.AddToViewport` _returnvalue 0)))))))

(event `self.ReceiveActorBeginOverlap`
  (params (OtherActor :type "Actor Object Reference"))
  ;[1 1 1] add/remove widget and enable/disable input if player haven't drank any drug
  (bind _asmain_character (cast `/Game/BluePrints/Actors/MainCharacter` OtherActor))
  (set `self.MainActor` _asmain_character)
  (if (not (>= (`/Game/BluePrints/Actors/MainCharacter.drugNumber` (`self.MainActor`)) 0))
    (bind _returnvalue (`|CreateWidget` "/Game/BluePrints/Widget/InteractKeyPrompt_E.InteractKeyPrompt_E_C"))
    (`UserWidget.AddToViewport` _returnvalue 0)
    (`self.EnableInput` (`GameplayStatics.GetPlayerController` 0))
    (goto _label :!via `Open`)))

(event `self.ReceiveActorEndOverlap`
  (params (OtherActor :type "Actor Object Reference"))
  ;[1 1 1] add/remove widget and enable/disable input if player haven't drank any drug
  (if (`KismetSystemLibrary.IsValid` (stale `self.ReceiveActorBeginOverlap` _returnvalue))
    (`Widget.RemoveFromParent` (stale `self.ReceiveActorBeginOverlap` _returnvalue)))
  (`self.DisableInput` (`GameplayStatics.GetPlayerController` 0))
  (goto _label :!via `Close`))

(event `SelectDrug`
  ;[1 1 1] Show durg selection widget when player clear the lock
  (bind _returnvalue (`|CreateWidget` "/Game/BluePrints/Widget/Switcher_drug_reserch.Switcher_drug_reserch_C"))
  (`/Game/BluePrints/Widget/Drug.setRefActors` (`/Game/BluePrints/Widget/Switcher_drug_reserch.Drug` _returnvalue) (`self.MainActor`) self _returnvalue)
  (`UserWidget.AddToViewport` _returnvalue 0))

(event `ShowDrugObtained`
  ;[1 1 1] Item Subtitle : You drank the drug... (Drug Obtained)
  (bind _returnvalue (`GameplayStatics.SpawnSound2D` "/Game/Assets/Audio/bottle.bottle" 1.0 1.0 0.0 null))
  (set `self.2dSound` _returnvalue)
  (bind _returnvalue_2 (`|CreateWidget` "/Game/BluePrints/Widget/Item_Subtitles.Item_Subtitles_C"))
  (`UserWidget.AddToViewport` _returnvalue_2 0)
  (`self.Item Subtitle Text`)
  (`KismetSystemLibrary.Delay` 4.0)
  (`Widget.RemoveFromParent` _returnvalue_2))

(event `Item Subtitle Text`
  ;[1 1 1] Item Subtitle : You drank the drug... (Drug Obtained)
  (`/Game/BluePrints/Widget/Item_Subtitles.DisplayItemLine` (stale `ShowDrugObtained` _returnvalue_2) "You drank the drug..."))

(fn `UserConstructionScript`)