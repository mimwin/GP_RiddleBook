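; BasicInteract is an interactable actor that toggles between two states on the Interact input while something overlaps it.
; Begin overlap shows an E-key prompt widget, enables input for player 0 and opens a Gate; end overlap reverses all three without checking which actor overlapped.
; Each gated press flips IsExecuted and calls the OnTrue or OnFalse custom event, both empty here.
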(event `InputAction|Interact`
  (params (Key :type "Key Structure"))
  ;[1 1 1] Press E Key to move
  (:`Pressed`
    ;[1 1 1] Open/Close Gate
    (`/Engine/EditorBlueprintResources/StandardMacros.Gate` true :!label _label
      (:`Exit`
        (if (`self.isExecuted`)
          (`self.OnTrue`)
          (set `self.isExecuted` false)
          (else
            (`self.OnFalse`)
            (set `self.isExecuted` true)))))))

(event `self.ReceiveActorBeginOverlap`
  (params (OtherActor :type "Actor Object Reference"))
  ;[1 1 1] add/remove widget and enable/disable input
  (bind _returnvalue (`|CreateWidget` "/Game/BluePrints/Widget/InteractKeyPrompt_E.InteractKeyPrompt_E_C"))
  (`UserWidget.AddToViewport` _returnvalue 0)
  (`self.EnableInput` (`GameplayStatics.GetPlayerController` 0))
  (goto _label :!via `Open`))

(event `self.ReceiveActorEndOverlap`
  (params (OtherActor :type "Actor Object Reference"))
  ;[1 1 1] add/remove widget and enable/disable input
  (`Widget.RemoveFromParent` (stale `self.ReceiveActorBeginOverlap` _returnvalue))
  (`self.DisableInput` (`GameplayStatics.GetPlayerController` 0))
  (goto _label :!via `Close`))

(event `OnTrue`
  ;[1 1 1] Define Custom Event!
)

(event `OnFalse`
  ;[1 1 1] Define Custom Event!
)

(fn `UserConstructionScript`)