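; Fireplace actor that serves as the game's ending trigger when the main character overlaps it.
; If the player has the key and a valid DrugNumber, it shows a success subtitle, plays unlock sounds, then shows one of four colour-variant credit widgets chosen by DrugNumber, with timed background music.
; Otherwise it shows an "It's not enough" subtitle, and leaving the overlap removes any subtitle widget.
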(event `self.ReceiveActorBeginOverlap`
  (params (OtherActor :type "Actor Object Reference"))
  (bind _mainactor (`self.MainActor`))
  (bind _asmain_character (cast `/Game/BluePrints/Actors/MainCharacter` OtherActor))
  (set `self.MainActor` _asmain_character)
  (if (and (`/Game/BluePrints/Actors/MainCharacter.isKeyObtained` _mainactor) (>= (`/Game/BluePrints/Actors/MainCharacter.drugNumber` _mainactor) 0))
    (bind _returnvalue (`|CreateWidget` "/Game/BluePrints/Widget/Subtitles.Subtitles_C"))
    (bind _output_get (set `self.SubtitlesWidgetRef` _returnvalue))
    (`UserWidget.AddToViewport` _output_get 0)
    (`self.True Subtitles Text`)
    (bind _returnvalue_2 (`GameplayStatics.SpawnSound2D` "/Game/Assets/Audio/Keysound_fireplace.Keysound_fireplace" 1.0 1.0 0.0 null))
    (set `self.2dSound` _returnvalue_2)
    (bind _returnvalue_3 (`GameplayStatics.SpawnSound2D` "/Game/Assets/Audio/opening_fireplace.opening_fireplace" 1.0 1.0 0.0 null))
    (set `self.2dSound` _returnvalue_3)
    (`KismetSystemLibrary.Delay` 0.5)
    (`Widget.RemoveFromParent` _output_get)
    (switch `int` (`/Game/BluePrints/Actors/MainCharacter.drugNumber` (`self.MainActor`))
      (:`0`
        ;[0 0 0] Display Credits
        (bind _returnvalue_4 (`|CreateWidget` "/Game/BluePrints/Widget/GameCredit_yellow.GameCredit_yellow_C"))
        (`UserWidget.AddToViewport` _returnvalue_4 0)
        (bind _returnvalue_5 (`GameplayStatics.SpawnSound2D` "/Game/Assets/Audio/Credit_BackGround.Credit_BackGround" 1.0 1.0 0.0 null))
        (set `self.2dSound` _returnvalue_5)
        (`KismetSystemLibrary.Delay` 10.0)
        (`AudioComponent.Stop` (`self.2dSound`)))
      (:`1`
        ;[0 0 0] Display Credits
        (bind _returnvalue_6 (`|CreateWidget` "/Game/BluePrints/Widget/GameCredit_orange.GameCredit_orange_C"))
        (`UserWidget.AddToViewport` _returnvalue_6 0)
        (bind _returnvalue_7 (`GameplayStatics.SpawnSound2D` "/Game/Assets/Audio/Credit_BackGround.Credit_BackGround" 1.0 1.0 0.0 null))
        (set `self.2dSound` _returnvalue_7)
        (`KismetSystemLibrary.Delay` 11.0)
        (`AudioComponent.Stop` (`self.2dSound`)))
      (:`2`
        ;[0 0 0] Display Credits
        (bind _returnvalue_8 (`|CreateWidget` "/Game/BluePrints/Widget/GameCredit_purple.GameCredit_purple_C"))
        (`UserWidget.AddToViewport` _returnvalue_8 0)
        (bind _returnvalue_9 (`GameplayStatics.SpawnSound2D` "/Game/Assets/Audio/Credit_BackGround.Credit_BackGround" 1.0 1.0 0.0 null))
        (set `self.2dSound` _returnvalue_9)
        (`KismetSystemLibrary.Delay` 10.0)
        (`AudioComponent.Stop` (`self.2dSound`)))
      (:`3`
        ;[0 0 0] Display Credits
        (bind _returnvalue_10 (`|CreateWidget` "/Game/BluePrints/Widget/GameCredit_green.GameCredit_green_C"))
        (`UserWidget.AddToViewport` _returnvalue_10 0)
        (bind _returnvalue_11 (`GameplayStatics.SpawnSound2D` "/Game/Assets/Audio/Credit_BackGround.Credit_BackGround" 1.0 1.0 0.0 null))
        (set `self.2dSound` _returnvalue_11)
        (`KismetSystemLibrary.Delay` 10.0)
        (`AudioComponent.Stop` (`self.2dSound`))))
    (else
      (bind _returnvalue_12 (`|CreateWidget` "/Game/BluePrints/Widget/Subtitles.Subtitles_C"))
      (bind _output_get_2 (set `self.SubtitlesWidgetRef` _returnvalue_12))
      (`UserWidget.AddToViewport` _output_get_2 0)
      (`self.Subtitles Text`))))

(event `True Subtitles Text`
  (`/Game/BluePrints/Widget/Subtitles.DisplayLine` (`self.SubtitlesWidgetRef`) "At Last..!"))

(event `Subtitles Text`
  (`/Game/BluePrints/Widget/Subtitles.DisplayLine` (`self.SubtitlesWidgetRef`) "It's not enough.."))

(event `self.ReceiveActorEndOverlap`
  (params (OtherActor :type "Actor Object Reference"))
  (bind _subtitleswidgetref (`self.SubtitlesWidgetRef`))
  (if (`KismetSystemLibrary.IsValid` _subtitleswidgetref)
    (`Widget.RemoveFromParent` _subtitleswidgetref)))

(fn `UserConstructionScript`)