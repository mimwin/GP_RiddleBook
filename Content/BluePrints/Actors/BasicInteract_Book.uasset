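; Interactable diary actor that shows a book page when the player presses Interact nearby.
; Overlap shows a subtitle and E-key prompt, enables input and opens a Gate; end overlap removes widgets and closes it.
; The gated key press toggles the BookPage widget via IsExecuted, showing a birthday-clue subtitle while open.
; Logic flagging the diary as opened on MainCharacter is present but never runs.
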(event `InputAction|Interact`
  (params (Key :type "Key Structure"))
  ;[1 1 1] Press E Key to move
  (:`Pressed`
    ;[1 1 1] Create Book page (widget)
    (`/Engine/EditorBlueprintResources/StandardMacros.Gate` true :!label _label
      (:`Exit`
        (if (`self.isExecuted`)
          (`self.OnTrue`)
          (set `self.isExecuted` false)
          (else
            (`self.OnFalse`)
            (set `self.isExecuted` true)))))))

(event `self.ReceiveActorBeginOverlap`
  (params (OtherActor :type "Actor Object Reference"))
  ;[1 1 1] add/remove widget and enable/disable input
  (`|ExecutionSequence`
    (:`then_0`
      ;[1 1 1] Subtitle - It looks like a diary
      (bind _returnvalue (`|CreateWidget` "/Game/BluePrints/Widget/Subtitles.Subtitles_C"))
      (bind _output_get (set `self.SubtitleWidgetRef` _returnvalue))
      (`self.Subtitle Text`)
      (`UserWidget.AddToViewport` _output_get 0))
    (:`then_1`
      (bind _returnvalue_2 (`|CreateWidget` "/Game/BluePrints/Widget/InteractKeyPrompt_E.InteractKeyPrompt_E_C"))
      (`UserWidget.AddToViewport` _returnvalue_2 0)
      (`self.EnableInput` (`GameplayStatics.GetPlayerController` 0))
      (goto _label :!via `Open`))))

(event `self.ReceiveActorEndOverlap`
  (params (OtherActor :type "Actor Object Reference"))
  ;[1 1 1] add/remove widget and enable/disable input
  (`Widget.RemoveFromParent` (`self.SubtitleWidgetRef`))
  (`|ExecutionSequence`
    (:`then_0`
      (if (`KismetSystemLibrary.IsValid` (stale `self.ReceiveActorBeginOverlap` _returnvalue_2))
        (`Widget.RemoveFromParent` (stale `self.ReceiveActorBeginOverlap` _returnvalue_2))
        (`Widget.RemoveFromParent` (`self.SubtitleWidgetRef`)))
      (`self.DisableInput` (`GameplayStatics.GetPlayerController` 0))
      (set `self.isExecuted` false)
      (goto _label :!via `Close`))
    (:`then_1`
      (if (`KismetSystemLibrary.IsValid` (stale `OnFalse` _returnvalue))
        (`Widget.RemoveFromParent` (stale `OnFalse` _returnvalue))
        (`Widget.RemoveFromParent` (`self.SubtitleWidgetRef2`))))))

(event `OnTrue`
  ;[1 1 1] Define Custom Event!
  (`Widget.RemoveFromParent` (stale `OnFalse` _returnvalue))
  (`Widget.RemoveFromParent` (`self.SubtitleWidgetRef2`)))

(event `OnFalse`
  ;[1 1 1] Define Custom Event!
  (bind _returnvalue (`|CreateWidget` "/Game/BluePrints/Widget/BookPage.BookPage_C"))
  (`UserWidget.AddToViewport` _returnvalue 0)
  ;[1 1 1] Adding subtitle while diary is open
  (`Widget.RemoveFromParent` (`self.SubtitleWidgetRef`))
  (bind _returnvalue_2 (`|CreateWidget` "/Game/BluePrints/Widget/Subtitles.Subtitles_C"))
  (bind _output_get (set `self.SubtitleWidgetRef2` _returnvalue_2))
  (`self.Subtitle Text 2`)
  (`UserWidget.AddToViewport` _output_get 0))

(event `Subtitle Text 2`
  ;[1 1 1] Subtitle " 12/10 must be somebody's birthday "
  (`/Game/BluePrints/Widget/Subtitles.DisplayLine` (`self.SubtitleWidgetRef2`) "12 / 10 must have been somebody's birthday."))

(event `Subtitle Text`
  ;[1 1 1] Subtitles - "It looks like a Diary. . . "
  (`/Game/BluePrints/Widget/Subtitles.DisplayLine` (`self.SubtitleWidgetRef`) "It looks like a Diary..."))

(fn `UserConstructionScript`)