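; Hand_hour is an interactable actor, apparently a clock's hour hand, that the player rotates in steps while overlapping it.
; Beginning overlap shows the InteractKeyPrompt_E widget, enables input and opens a Gate, and ending overlap reverses all three.
; Pressing X (not E, despite the widget's name) passes through the Gate to add a fixed roll increment and print debug text.
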(event `self.ReceiveActorBeginOverlap`
  (params (OtherActor :type "Actor Object Reference"))
  (bind _returnvalue (`KismetMathLibrary.MakeRotator` (+ (.roll (`self.K2_GetActorRotation`)) 50.0) (.pitch (`self.K2_GetActorRotation`)) (.yaw (`self.K2_GetActorRotation`))))
  ;[1 1 1] add/remove widget and enable/disable input
  (bind _returnvalue_2 (`|CreateWidget` "/Game/BluePrints/Widget/InteractKeyPrompt_E.InteractKeyPrompt_E_C"))
  (`UserWidget.AddToViewport` _returnvalue_2 0)
  (`self.EnableInput` (`GameplayStatics.GetPlayerController` 0))
  (goto _label :!via `Open`))

(event `Key|X`
  (params (Key :type "Key Structure"))
  (bind _returnvalue (`KismetMathLibrary.MakeRotator` (+ (.roll (`self.K2_GetActorRotation`)) 50.0) (.pitch (`self.K2_GetActorRotation`)) (.yaw (`self.K2_GetActorRotation`))))
  (:`Pressed`
    (`/Engine/EditorBlueprintResources/StandardMacros.Gate` true :!label _label
      (:`Exit`
        (`self.K2_SetActorRotation` _returnvalue)
        (`KismetSystemLibrary.PrintText` "Hello")
        (`KismetSystemLibrary.PrintText` (`KismetTextLibrary.Conv_RotatorToText` _returnvalue))))))

(event `self.ReceiveActorEndOverlap`
  (params (OtherActor :type "Actor Object Reference"))
  ;[1 1 1] add/remove widget and enable/disable input
  (`Widget.RemoveFromParent` (stale `self.ReceiveActorBeginOverlap` _returnvalue_2))
  (`self.DisableInput` (`GameplayStatics.GetPlayerController` 0))
  (goto _label :!via `Close`))

(fn `UserConstructionScript`)